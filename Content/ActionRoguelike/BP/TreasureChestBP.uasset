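; Treasure chest interactable Blueprint, apparently over a native parent that supplies the interaction logic.
; Interact calls the parent implementation and prints a debug message, while Tick prints the LidOpened state every frame.
; Two disconnected chains never run: a RequiredKeyCard gameplay tag check on an SActionComponent, and a FlipFlop timeline that pitches the lid open or closed and activates particles on finish.
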(event EventTick
  (params (DeltaSeconds :type Float%20%28single-precision%29))
  (Development|PrintString (Utilities|String|Append "Lid Opened:" (Utilities|String|ToString(Boolean) (Variables|Default|GetbLidOpened))) true true "(R=0.000000,G=1.000000,B=0.268480,A=1.000000)" 0.0))

(event EventInteract
  (params (InstigatorPawn :type Pawn%20Object%20Reference))
  (|CallParentFunction InstigatorPawn)
  (Development|PrintString "Treasure Chest Interact (BP)" true true "(R=0.000000,G=0.036073,B=1.000000,A=1.000000)"))

(fn ConstructionScript)